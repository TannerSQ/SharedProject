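; Master enemy Blueprint whose EnemyBehaviour settings drive how it wakes, moves and picks player targets.
; Sight overlap, damage or a trigger activates it by aggravation type, setting the target, enlarging the detection sphere and updating level camera weights if enabled.
; While active, Tick line-traces to track visible in-range targets and runs delayed retargeting to closest or random players.
; Reached moves lead to searching nearby or roaming; deactivation logic is unwired.
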(event `self.ReceiveBeginPlay`
  ;[0 0 0 1 12] Enable Character
  (`self.SpawnDefaultController`))

(event `self.DetectionSphere.OnComponentBeginOverlap`
  (params (OverlappedComponent :type "PrimitiveComponent Object Reference") (OtherActor :type "Actor Object Reference") (OtherComp :type "PrimitiveComponent Object Reference") (OtherBodyIndex :type Integer) (bFromSweep :type Boolean) (SweepResult :type "HitResult Structure (by ref)"))
  ;[0 0 0] Activation: Sight overlap
  (if (and (!= OtherActor self) (`self.ActorHasTag` OtherActor "PlayerOwned"))
    ;[0 0 0] Can be activated by sight?
    (if (`|EnumEquality` (`.Aggrevation_11_5E5E2F834C5C172334DAE58FE871726E` (break `/Game/Blueprints/Variables/Struct/Enemy/Struct_EnemyBehaviour` (`self.EnemyBehaviour`))) "NewEnumerator1")
      ;[0 0 0] Activate
      (if (not (`self.bActivated`))
        (`self.AI: Activate Enemy` OtherActor)))))

(event `/Game/Blueprints/Variables/Interfaces/Interface_Gameplay.Combat: Damage`
  (params (Damage :type "/Game/Blueprints/Variables/Struct/Damage/Struct_Damage Structure") (Actor :type "Actor Object Reference"))
  ;[0 0 0] Activation: Attacked
  (`/Game/Blueprints/Components/Component_Health.Combat: Damage` (`self.Component_Health`) Damage null)
  ;[0 0 0] Can be activated by combat?
  (if (`|EnumEquality` (`.Aggrevation_11_5E5E2F834C5C172334DAE58FE871726E` (break `/Game/Blueprints/Variables/Struct/Enemy/Struct_EnemyBehaviour` (`self.EnemyBehaviour`))) "NewEnumerator0")
    ;[0 0 0] Activate
    (if (not (`self.bActivated`))
      (`self.AI: Activate Enemy` Actor))))

(event `/Game/Blueprints/Variables/Interfaces/Interface_Gameplay.Trigger`
  (params (Trigger :type "Actor Object Reference"))
  ;[0 0 0] Can be activated by combat?
  (if (`|EnumEquality` (`.Aggrevation_11_5E5E2F834C5C172334DAE58FE871726E` (break `/Game/Blueprints/Variables/Struct/Enemy/Struct_EnemyBehaviour` (`self.EnemyBehaviour`))) "NewEnumerator2")
    ;[0 0 0] Activate
    (if (not (`self.bActivated`))
      (`self.AI: Activate Enemy` Trigger))))

(event `AI: Player Location Hint`
  (if (`self.Target in Range`)
    (bind _randomlocation (`NavigationSystemV1.K2_GetRandomLocationInNavigableRadius` (`self.K2_GetActorLocation` (`self.Current Target`)) 300.0 null null))
    (`|AIMoveTo` self _randomlocation null 150.0
      (:`OnSuccess`
        (`self.AI: Player Location Hint`)))
    (else
      (`self.AI: Idle Roaming`))))

(event `self.ReceiveTick`
  (params (DeltaSeconds :type "Float (single-precision)"))
  ;[0 0 0] Event Tick
  (if (`self.bActivated`)
    (`|ExecutionSequence`
      (:`then_0`
        ;[0 0 0] Is Target Valid?
        (if (`KismetSystemLibrary.IsValid` (`self.Current Target`))
          ;[0 0 0] Can Enemy see Target?
          (bind _outhit (`KismetSystemLibrary.LineTraceSingle` :`Start` (`SceneComponent.K2_GetComponentLocation` (`self.CapsuleComponent`)) :`End` (`self.K2_GetActorLocation` (`self.Current Target`)) :`TraceChannel` "TraceTypeQuery1" :`DrawDebugType` "ForOneFrame"))
          (set `self.Target in View` (== (`self.Current Target`) (`.HitActor` (`GameplayStatics.BreakHitResult` _outhit))))
          (set `self.Target in Range` (<= (`self.GetDistanceTo` (`.HitActor` (`GameplayStatics.BreakHitResult` _outhit))) (`.AwakeAggrevationRadius_34_7E7294C545BF5CAE5A397B9ED87EF15E` (break `/Game/Blueprints/Variables/Struct/Enemy/Struct_EnemyBehaviour` (`self.EnemyBehaviour`)))))
          (if (and (`self.Target in View`) (`self.Target in Range`))
            (set `self.Last Seen Target Location` (`.ImpactPoint` (`GameplayStatics.BreakHitResult` _outhit))))
          ;[0 0 0] Movement Archetype
          (switch `/Game/Blueprints/Variables/Enum/Enum_EnemyBehaviour_Movement` (`.Movement_24_C389A71346DB6AFA8D1BA3BBFB87E71B` (break `/Game/Blueprints/Variables/Struct/Enemy/Struct_EnemyBehaviour` (`self.EnemyBehaviour`)))
            (:`NewEnumerator0`
              (if (and (`self.Target in Range`) (`self.Target in View`))
                (`|AIMoveTo` self (`self.K2_GetActorLocation` (`self.Current Target`)) null 150.0
                  (:`OnSuccess`
                    (`self.AI: Player Location Hint`))))))))
      (:`then_1`
        (switch `/Game/Blueprints/Variables/Enum/Enemy/Enum_EnemyBehaviour_Focusing` (`.Focusing_4_7DA19533466AA1A7CF2C548F97427E45` (break `/Game/Blueprints/Variables/Struct/Enemy/Struct_EnemyBehaviour` (`self.EnemyBehaviour`)))
          (:`NewEnumerator0`
            ;[0 0 0] New Target: Closest Player
            (`KismetSystemLibrary.Delay` (`self.Calculate: Attention Span`) :!label _label)
            (bind _players (`self.Get: Closest Player in Range`))
            (set `self.Current Target` _players)
            (goto _label))
          (:`NewEnumerator2`
            ;[0 0 0] New Target: Random Player in sight
            (`KismetSystemLibrary.Delay` (`self.Calculate: Attention Span`) :!label _label_2)
            (bind (_found _players_2) (`self.Get: Players in Range`))
            (if _found
              (set `self.Current Target` (`|GetArrayItem` _players_2 (`KismetMathLibrary.RandomIntegerInRange` 0 (- (`KismetArrayLibrary.Array_Length` _players_2) 1))))
              (goto _label_2))))))))

(event `AI: Idle Roaming`
  (bind _randomlocation (`NavigationSystemV1.K2_GetRandomLocationInNavigableRadius` (`self.K2_GetActorLocation`) 500.0 null null))
  (`|AIMoveTo` self _randomlocation null 150.0
    (:`OnSuccess`
      (`KismetSystemLibrary.Delay` 1.5)
      (`self.AI: Idle Roaming`))))

(fn `AI: Activate Enemy`
  (params (`Actor (If Applicable)` :type "Actor Object Reference"))
  (locals (Actor :type "Actor Object Reference"))
  ;[0 0 0] Get Actor
  (set `local.Actor` `Actor (If Applicable)`)
  ;[0 0 0] Get Target (Currently the Activator)
  (set `self.Current Target` (`local.Actor`))
  ;[0 0 0] Set Activated
  (set `self.bActivated` true)
  (`self.AI: Enemy Alert Status` true))

(fn `AI: Deactivate Enemy`
  (params (`Idle Roam` :type Boolean))
  (set `self.bActivated` false)
  (`/Game/Blueprints/Camera/Camera_Default.Camera: Update Weights` (`/Game/Blueprints/Core/GM_Default.Level Camera` (cast `/Game/Blueprints/Core/GM_Default` (`GameplayStatics.GetGameMode`) :!pure true)) false self)
  (if `Idle Roam`
    (`self.AI: Idle Roaming`)))

(fn `AI: Enemy Alert Status`
  (params (Alert :type Boolean))
  (locals (AlertStatus :type Boolean))
  (bind ((`IdleAggrevationRadius_33_4B698214453CA56110986C8F2EC7CEA6` _idleaggrevationradius) (`AwakeAggrevationRadius_34_7E7294C545BF5CAE5A397B9ED87EF15E` _awakeaggrevationradius)) (break `/Game/Blueprints/Variables/Struct/Enemy/Struct_EnemyBehaviour` (`self.EnemyBehaviour`)))
  (set `local.AlertStatus` Alert)
  ;[0 0 0] Does Enemy affect Camera?
  (if (`/Game/Blueprints/Components/Component_CameraWeight.Active` (`self.Component_CameraWeight`))
    (`/Game/Blueprints/Camera/Camera_Default.Camera: Update Weights` (`/Game/Blueprints/Core/GM_Default.Level Camera` (cast `/Game/Blueprints/Core/GM_Default` (`GameplayStatics.GetGameMode`) :!pure true)) (`local.AlertStatus`) self)
    ;[0 0 0] Enemy is awake! Be more alert
    (`SphereComponent.SetSphereRadius` (`self.DetectionSphere`) (select `bool` (`local.AlertStatus`) :`false` _idleaggrevationradius :`true` _awakeaggrevationradius) true)))

(fn `AI: Get New Target`
  (params (`Always Switch Target` :type Boolean)))

(fn `Get: Closest Player in Range`
  (returns (Players :type "/Game/Blueprints/Character/CH_Default Object Reference"))
  (locals (PlayersInSight :type "Array of /Game/Blueprints/Character/CH_Default Object Reference") (ClosestDistance :type "Float (double-precision)") (ClosestPlayer :type "/Game/Blueprints/Character/CH_Default Object Reference"))
  (set `local.ClosestDistance` 99999.0)
  (set `local.ClosestPlayer` null)
  (bind _outactors (`GameplayStatics.GetAllActorsOfClass` "/Game/Blueprints/Character/CH_Default.CH_Default_C"))
  (for _array_element _outactors
    (bind _returnvalue (`self.GetDistanceTo` _array_element self))
    (if (< _returnvalue (`local.ClosestDistance`))
      (set `local.ClosestDistance` _returnvalue)
      (set `local.ClosestPlayer` (cast `/Game/Blueprints/Character/CH_Default` _array_element :!pure true))))
  (return (`local.ClosestPlayer`)))

(fn `Get: Players in Range`
  (returns (Found :type Boolean) (Players :type "Array of /Game/Blueprints/Character/CH_Default Object Reference"))
  (locals (PlayersInSight :type "Array of /Game/Blueprints/Character/CH_Default Object Reference"))
  (bind _playersinsight (`local.PlayersInSight`))
  (bind _outactors (`GameplayStatics.GetAllActorsOfClass` "/Game/Blueprints/Character/CH_Default.CH_Default_C"))
  (for _array_element _outactors
    (bind (_asch_default _bsuccess) (cast `/Game/Blueprints/Character/CH_Default` _array_element :!pure true))
    (if (and _bsuccess (<= (`self.GetDistanceTo` _array_element self) (`.AwakeAggrevationRadius_34_7E7294C545BF5CAE5A397B9ED87EF15E` (break `/Game/Blueprints/Variables/Struct/Enemy/Struct_EnemyBehaviour` (`self.EnemyBehaviour`)))))
      (`KismetArrayLibrary.Array_Add` (`local.PlayersInSight`) _asch_default)))
  (return (!= (`KismetArrayLibrary.Array_Length` _playersinsight) 0) _playersinsight))

(fn `UserConstructionScript`
  (bind _enemybehaviour_idleaggrevationradius (break `/Game/Blueprints/Variables/Struct/Enemy/Struct_EnemyBehaviour` (`self.EnemyBehaviour`)))
  (`SphereComponent.SetSphereRadius` (`self.DetectionSphere`) _enemybehaviour_idleaggrevationradius true))