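; Default player character driven by controller interface events, with twin-stick movement and aim, a cooldown-gated dash and sword melee.
; A Rotation component turns independently of the capsule, following stick input or a locked-on target chosen by sphere trace and smallest yaw offset.
; Melee damages overlapping actors; incoming damage feeds the health component and launches the character away from the attacker.
; Tick drives cosmetic lean and bobbing timelines from movement acceleration.
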(event `/Game/Blueprints/Variables/Interfaces/Interface_Gameplay.Combat: Melee Swing`
  (for _array_element (`PrimitiveComponent.GetOverlappingActors` (`self.Melee_HitCollision`) null)
    (message `/Game/Blueprints/Variables/Interfaces/Interface_Gameplay.Combat: Damage` _array_element (make `/Game/Blueprints/Variables/Struct/Damage/Struct_Damage` 15.0 200.0) self)))

(event `/Game/Blueprints/Variables/Interfaces/Interface_Gameplay.Controller: Send Left Face Button`
  (params (Pressed :type Boolean))
  (set `/Game/Assets/Weaponry/Sword/AnimBP_Sword.Activate` Pressed (cast `/Game/Assets/Weaponry/Sword/AnimBP_Sword` (`SkeletalMeshComponent.GetAnimInstance` (`self.SM_Sword`)) :!pure true)))

(event `self.ReceiveBeginPlay`
  (`self.SpawnDefaultController`))

(event `/Game/Blueprints/Variables/Interfaces/Interface_Gameplay.Setup`
  (params (Controller :type "/Game/Blueprints/Core/PC_Default Object Reference"))
  (set `self.Player Controller` Controller)
  (`self.Setup Variables`))

(event `/Game/Blueprints/Variables/Interfaces/Interface_Gameplay.Controller: Send Left Joystick`
  (params (Input :type "Vector2D Structure"))
  (bind _output_get (set `self.Controller: Movement` Input))
  (`self.Character Movement` _output_get))

(event `/Game/Blueprints/Variables/Interfaces/Interface_Gameplay.Controller: Send Dash`
  (`self.Character Dash` (`self.Dash: Strength`))
  (if (not (`self.Dash: Cooldown`))
    (`KismetSystemLibrary.Delay` 3.0)
    (set `self.Dash: Cooldown` true)))

(event `/Game/Blueprints/Variables/Interfaces/Interface_Gameplay.Controller: Send Right Joystick`
  (params (Input :type "Vector2D Structure"))
  (bind _output_get (set `self.Controller: Orientation` Input))
  (`self.Character Orientation` _output_get)
  (if (not (`self.Is Player Rotating`))
    (`KismetSystemLibrary.RetriggerableDelay` 1.5)
    (`self.Focus Entity` false)))

(event `/Game/Blueprints/Variables/Interfaces/Interface_Gameplay.Players: Stop Moving`
  (params (Pause :type Boolean))
  (set `self.Pause Players` Pause))

(event `/Game/Blueprints/Variables/Interfaces/Interface_Gameplay.Killzone`
  (`/Game/Blueprints/Core/PC_Default.Player: Leave` (`self.Player Controller`)))

(event `self.ReceiveTick`
  (params (DeltaSeconds :type "Float (single-precision)"))
  (bind (_relativelocation_x _relativelocation_y _relativelocation_z) (`KismetMathLibrary.BreakVector` (`SceneComponent.RelativeLocation` (`self.Rotation`))))
  ;[1 0 0 0.25] Bad.
  (`|ExecutionSequence`
    (:`then_1`
      (if (`KismetMathLibrary.NearlyEqual_FloatFloat` (`KismetMathLibrary.VSize` (`CharacterMovementComponent.GetCurrentAcceleration` (`self.CharacterMovement`))) 0.0 350.0)
        (`|ExecutionSequence`
          (:`then_0`
            (bind (_direction _lerp) (`Timeline|Lean` :!via `Reverse` :!label _label)
              (:`Update`
                (`SceneComponent.K2_SetRelativeRotation` (`self.LeanRotation`) (`KismetMathLibrary.MakeRotator` 0.0 (`KismetMathLibrary.Lerp` 0.0 15.0 _lerp)) false false))))
          (:`then_1`
            (`|ExecutionSequence`
              (:`then_0`
                (bind (_direction_2 _lerp_2) (`Timeline|Bobbing` :!via `Stop` :!label _label_2)
                  (:`Update`
                    (`SceneComponent.K2_SetRelativeLocation` (`self.Rotation`) (`KismetMathLibrary.MakeVector` 0.0 0.0 (`KismetMathLibrary.Lerp` -60.0 -40.0 _lerp_2)) false false))))
              (:`then_1`
                (bind (_direction_3 _lerp_3) (`Timeline|Timeline_0` :!via `PlayFromStart`)
                  (:`Update`
                    (`SceneComponent.K2_SetRelativeLocation` (`self.Rotation`) (`KismetMathLibrary.MakeVector` 0.0 0.0 (`KismetMathLibrary.Lerp` _relativelocation_z -60.0 _lerp_3)) false false)))))))
        (else
          (`|ExecutionSequence`
            (:`then_0`
              (goto _label))
            (:`then_1`
              (goto _label_2))))))))

(event `/Game/Blueprints/Variables/Interfaces/Interface_Gameplay.Combat: Damage`
  (params (Damage :type "/Game/Blueprints/Variables/Struct/Damage/Struct_Damage Structure") (Actor :type "Actor Object Reference"))
  (bind (_returnvalue_x _returnvalue_y) (`KismetMathLibrary.BreakVector` (* (`KismetMathLibrary.Conv_RotatorToVector` (`KismetMathLibrary.FindLookAtRotation` (`self.K2_GetActorLocation` (`self.Last Player to Damage`)) (`self.K2_GetActorLocation` self))) (`.Knockback_14_3CE07B1A483C74273B39F2A48E33E5D2` (break `/Game/Blueprints/Variables/Struct/Damage/Struct_Damage` Damage)))))
  ;[0 0 0] Recieve Damage from Enemy
  (set `self.Last Player to Damage` Actor)
  ;[0 0 0] Send Damage to Health Component
  (`/Game/Blueprints/Components/Component_Health.Combat: Damage` (`self.Component_Health`) Damage null)
  (`self.LaunchCharacter` (`KismetMathLibrary.MakeVector` _returnvalue_x _returnvalue_y 150.0)))

(event `/Game/Blueprints/Variables/Interfaces/Interface_Gameplay.Combat: Health Depleted`)

(event `/Game/Blueprints/Variables/Interfaces/Interface_Gameplay.Controller: Send Lock-On`
  (params (Pressed :type Boolean))
  (if Pressed
    (if (not (`self.Focus Mode`))
      (bind (_found _entities) (`self.Get Focusable Entities` (`self.Focus Radius`)))
      (if _found
        (bind _entity (`self.Get Closest in View` _entities))
        (`self.Focus Entity` true _entity))
      (else
        (`self.Focus Entity` false)))))

(fn `Character Dash`
  (params (Strength :type "Float (double-precision)"))
  (bind _returnvalue (`CharacterMovementComponent.GetCurrentAcceleration` (`self.CharacterMovement`)))
  (if (`self.Pause Players`)
    _
    (elif (`self.Dash: Cooldown`)
      (`self.LaunchCharacter` (* (select `bool` (`KismetMathLibrary.NearlyEqual_FloatFloat` (`KismetMathLibrary.VSize` _returnvalue) 0.0 1.0) :`false` (`KismetMathLibrary.GetForwardVector` (`KismetMathLibrary.Conv_VectorToRotator` _returnvalue)) :`true` (`SceneComponent.GetForwardVector` (`self.Arrow1`))) Strength) true true)
      (set `self.Dash: Cooldown` false))))

(fn `Character Movement`
  (params (Input :type "Vector2D Structure"))
  (locals (`Input X` :type "Float (double-precision)" :default 0.0) (`Input Y` :type "Float (double-precision)"))
  (set `local.Input X` Input_X)
  (set `local.Input Y` Input_Y)
  (if (not (`self.Pause Players`))
    (`self.AddMovementInput` (`SceneComponent.GetRightVector` (`self.CapsuleComponent`)) (`local.Input X`))
    (`self.AddMovementInput` (`SceneComponent.GetForwardVector` (`self.CapsuleComponent`)) (`local.Input Y`))))

(fn `Character Orientation`
  (params (Input :type "Vector2D Structure"))
  (locals (Local_Input :type "Vector2D Structure"))
  (bind (_input_x _input_y) (`KismetMathLibrary.BreakVector2D` (`local.Input`)))
  (bind (_input_x_2 _input_y_2) (`KismetMathLibrary.BreakVector2D` (`local.Input`)))
  (bind (_controller__movement_x _controller__movement_y) (`KismetMathLibrary.BreakVector2D` (`self.Controller: Movement`)))
  (bind (_returnvalue_roll _returnvalue_pitch _returnvalue_yaw) (`KismetMathLibrary.BreakRotator` (`KismetMathLibrary.FindLookAtRotation` (`self.K2_GetActorLocation`) (`self.K2_GetActorLocation` (`self.Focused Entity`)))))
  (if (`self.Pause Players`)
    _
    (elif (not (`self.Focus Mode`))
      (if (not (`self.Is Player Rotating`))
        (if (not (`KismetMathLibrary.NearlyEqual_FloatFloat` (`KismetMathLibrary.VSize2D` (`self.Controller: Movement`)) 0.0 0.35))
          (`SceneComponent.K2_SetWorldRotation` (`self.Rotation`) (`KismetMathLibrary.Conv_VectorToRotator` (`KismetMathLibrary.MakeVector` _controller__movement_y _controller__movement_x)) false false))
        (else
          (`SceneComponent.K2_SetWorldRotation` (`self.Rotation`) (`KismetMathLibrary.Conv_VectorToRotator` (`KismetMathLibrary.MakeVector` (* _input_y_2 -1.0) _input_x_2)) false false)))
      (elif (not (`self.Is Player Rotating`))
        (`/Engine/EditorBlueprintResources/StandardMacros.IsValid` (`self.Focused Entity`)
          (:`Is Valid`
            (`SceneComponent.K2_SetWorldRotation` (`self.Rotation`) (`KismetMathLibrary.MakeRotator` 0.0 0.0 _returnvalue_yaw) false false))
          (:`Is Not Valid`
            (`self.Focus Entity` false)))
        (else
          (`SceneComponent.K2_SetWorldRotation` (`self.Rotation`) (`KismetMathLibrary.Conv_VectorToRotator` (`KismetMathLibrary.MakeVector` (* _input_y -1.0) _input_x)) false false)
          (bind (_found _entities) (`self.Get Focusable Entities` (`self.Focus Radius`)))
          (if _found
            (bind _entity (`self.Get Closest in View` _entities))
            (`self.Focus Entity` true _entity)))))))

(fn `Focus Entity`
  (params (Enable :type Boolean) (Actor :type "Actor Object Reference"))
  (set `self.Focused Entity` (`local.Actor`))
  (set `self.Focus Mode` (`local.Enable`)))

(fn `Get Closest in View`
  (params (`Actor Array` :type "Array of Actor Object Reference"))
  (returns (Entity :type "Actor Object Reference"))
  (locals (ClosestFloat :type "Float (double-precision)" :default 2.0) (ClosestActor :type "Actor Object Reference"))
  (set `local.ClosestFloat` 2.0)
  (for _array_element `Actor Array`
    (bind (_returnvalue_roll _returnvalue_pitch _returnvalue_yaw) (`KismetMathLibrary.BreakRotator` (`KismetMathLibrary.ComposeRotators` (`KismetMathLibrary.FindLookAtRotation` (`self.K2_GetActorLocation`) (`self.K2_GetActorLocation` _array_element)) (* (`SceneComponent.K2_GetComponentRotation` (`self.Rotation`)) -1.0))))
    (bind _returnvalue (`KismetMathLibrary.FClamp` (`KismetMathLibrary.Abs` (/ _returnvalue_yaw 180.0))))
    (if (< _returnvalue (`local.ClosestFloat`))
      (set `local.ClosestFloat` _returnvalue)
      (set `local.ClosestActor` _array_element)))
  (return (`local.ClosestActor`)))

(fn `Get Focusable Entities`
  (params (Radius :type "Float (double-precision)") (`Infront of player` :type Boolean))
  (returns (Found :type Boolean) (Entities :type "Array of Actor Object Reference") (Random :type "Actor Object Reference"))
  (locals (L_Entities :type "Array of Actor Object Reference"))
  (bind _l_entities (`local.L_Entities`))
  (bind _returnvalue (select `bool` (not `Infront of player`) :`false` (+ (`SceneComponent.K2_GetComponentLocation` (`self.CapsuleComponent`)) (* (`SceneComponent.GetForwardVector` (`self.Arrow1`)) Radius)) :`true` (`SceneComponent.K2_GetComponentLocation` (`self.CapsuleComponent`))))
  (bind _outhits (`KismetSystemLibrary.SphereTraceMultiForObjects` _returnvalue _returnvalue Radius (`|MakeArray` "ObjectTypeQuery8" :!type "EObjectTypeQuery Enum") false (`|MakeArray` self :!type "Actor Object Reference") "None" true (struct :`R` 1.0 :`A` 1.0) (struct :`G` 1.0 :`A` 1.0) 0.3))
  (for _array_element _outhits
    (if (`KismetSystemLibrary.IsValid` (`self.GetComponentByClass` (`.HitActor` (`GameplayStatics.BreakHitResult` _array_element)) "/Game/Blueprints/Components/Component_Focusable.Component_Focusable_C"))
      (`KismetArrayLibrary.Array_Add` (`local.L_Entities`) (`.HitActor` (`GameplayStatics.BreakHitResult` _array_element)))))
  (return (not (== (`KismetArrayLibrary.Array_Length` (`local.L_Entities`)) 0)) (`local.L_Entities`) (`|GetArrayItem` _l_entities (`KismetMathLibrary.RandomIntegerInRange` 0 (- (`KismetArrayLibrary.Array_Length` _l_entities) 1)))))

(fn `Setup Variables`
  (set `/Game/Blueprints/Components/Component_Health.Stats` (`.Stats_11_969629254522C927519F4692E73B95D7` (break `/Game/Blueprints/Variables/Struct/Player/Struct_PlayerInfo` (`/Game/Blueprints/Core/PC_Default.Player Info` (`self.Player Controller`)))) (`self.Component_Health`))
  (`/Game/UI/Players/Player_CharacterTitle.Set Title` (cast `/Game/UI/Players/Player_CharacterTitle` (`WidgetComponent.GetUserWidgetObject` (`self.Character Title`)) :!pure true) (`.Title_12_50CF248541E96F9EE0914C958BB99068` (break `/Game/Blueprints/Variables/Struct/Player/Struct_PlayerInfo` (`/Game/Blueprints/Core/PC_Default.Player Info` (`self.Player Controller`))))))

(fn `UserConstructionScript`)