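; BP_CameraFocus is a trigger volume that temporarily focuses the level camera on a point when a CH_Default character enters its box.
; LevelSetupComplete caches the LevelCamera from GM_Default and prints a debug string.
; On overlap, it passes the CameraFocusLocation component's world position to that camera and turns on FocusCameraOnLocation, then turns it off after a Time delay.
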(event `/Game/Blueprints/Variables/Interfaces/Interface_General.Level Setup Complete`
  (bind _asgm_default (cast `/Game/Blueprints/Core/GM_Default` (`GameplayStatics.GetGameMode`)))
  (set `self.Player Camera` (`/Game/Blueprints/Core/GM_Default.Level Camera` _asgm_default))
  (`KismetSystemLibrary.PrintString` "Hello"))

(event `self.Box.OnComponentBeginOverlap`
  (params (OverlappedComponent :type "PrimitiveComponent Object Reference") (OtherActor :type "Actor Object Reference") (OtherComp :type "PrimitiveComponent Object Reference") (OtherBodyIndex :type Integer) (bFromSweep :type Boolean) (SweepResult :type "HitResult Structure (by ref)"))
  (cast `/Game/Blueprints/Character/CH_Default` OtherActor)
  (set `/Game/Blueprints/Camera/Camera_Default.Location_CameraFocus` (`SceneComponent.K2_GetComponentLocation` (`self.Camera Focus Location`)) (`self.Player Camera`))
  (set `/Game/Blueprints/Camera/Camera_Default.Focus Camera on Location` true (`self.Player Camera`))
  (`KismetSystemLibrary.Delay` (`self.Time`))
  (set `/Game/Blueprints/Camera/Camera_Default.Focus Camera on Location` false (`self.Player Camera`)))

(fn `UserConstructionScript`)