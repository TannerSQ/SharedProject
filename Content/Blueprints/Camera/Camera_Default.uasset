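; Shared multiplayer camera that frames all joined players, with optional pull toward weighted actors such as enemies.
; Events maintain the player and weighted-actor lists, summing each weight component into a clamped blend alpha.
; Tick moves the CameraOffset arm between both groups' bounds centers and maps player spread through a curve to both arm lengths.
; A focus flag overrides this, moving the camera to a set location at a fixed distance.
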(event `Camera: Update Players`
  (params (Add :type Boolean) (Actor :type "Actor Object Reference"))
  (bind _joined_playeractors (`self.Joined_PlayerActors`))
  ;[0 0 0] Update Players Variable
  (if Add
    (`KismetArrayLibrary.Array_Add` _joined_playeractors Actor)
    (else
      (`KismetArrayLibrary.Array_RemoveItem` _joined_playeractors Actor))))

(event `Camera: Update Weights`
  (params (Add :type Boolean) (Actor :type "Actor Object Reference"))
  (bind _joined_weightedactors (`self.Joined_WeightedActors`))
  ;[0 0 0] Update Enemies Variable & Weights
  (if Add
    (`KismetArrayLibrary.Array_Add` _joined_weightedactors Actor)
    (else
      (`KismetArrayLibrary.Array_RemoveItem` _joined_weightedactors Actor)))
  (set `self.Camera_WeightedActors_Weights` 0.0)
  (for _array_element (`self.Joined_WeightedActors`)
    (set `self.Camera_WeightedActors_Weights` (`KismetMathLibrary.FClamp` (+ (`self.Camera_WeightedActors_Weights`) (`/Game/Blueprints/Components/Component_CameraWeight.Weight` (`self.GetComponentByClass` _array_element "/Game/Blueprints/Components/Component_CameraWeight.Component_CameraWeight_C")))))))

(event `self.ReceiveTick`
  (params (DeltaSeconds :type "Float (single-precision)"))
  (bind _returnvalue (`CurveFloat.GetFloatValue` (`self.Camera_DistanceCurve`) (/ (- (`KismetMathLibrary.FClamp` (`KismetMathLibrary.VSize` (`self.Players_CameraExtent`)) (`self.Camera_PlayerMinDistance`) (`self.Camera_PlayerMaxDistance`)) (`self.Camera_PlayerMinDistance`)) (- (`self.Camera_PlayerMaxDistance`) (`self.Camera_PlayerMinDistance`)))))
  ;[0 0 0] Players Exist?
  (if (> (`KismetArrayLibrary.Array_Length` (`self.Joined_PlayerActors`)) 0)
    (if (`self.Focus Camera on Location`)
      (`SceneComponent.K2_SetWorldLocation` (`self.CameraOffset`) (`self.Location_CameraFocus`) false false)
      (set `SpringArmComponent.TargetArmLength` 900.0 (`self.CameraDistance`))
      (else
        ;[0 0 0] Players Camera Variables
        (bind (_center _boxextent) (`GameplayStatics.GetActorArrayBounds` (`self.Joined_PlayerActors`) true))
        (set `self.Players_AverageLocation` _center)
        (set `self.Players_CameraExtent` _boxextent)
        ;[0 0 0] Update Camera Location
        (bind _center_2 (`GameplayStatics.GetActorArrayBounds` (`self.Joined_WeightedActors`) true))
        (`SceneComponent.K2_SetWorldLocation` (`self.CameraOffset`) (select `bool` (> (`KismetArrayLibrary.Array_Length` (`self.Joined_WeightedActors`)) 0) :`false` (`self.Players_AverageLocation`) :`true` (`KismetMathLibrary.MakeVector` (.x (select `bool` (> (`self.Camera_WeightedActors_Weights`) 0.0) :`false` (`self.Players_AverageLocation`) :`true` (`KismetMathLibrary.VLerp` (`self.Players_AverageLocation`) _center_2 (`self.Camera_WeightedActors_Weights`)))) (.y (select `bool` (> (`self.Camera_WeightedActors_Weights`) 0.0) :`false` (`self.Players_AverageLocation`) :`true` (`KismetMathLibrary.VLerp` (`self.Players_AverageLocation`) _center_2 (`self.Camera_WeightedActors_Weights`)))))) false false)
        ;[0 0 0] Camera Zooming
        (bind _output_get (set `self.Camera_ArmDistance_Players` (`KismetMathLibrary.Lerp` (`self.Camera_MinDistance`) (`self.Camera_MaxDistance`) _returnvalue)))
        (set `SpringArmComponent.TargetArmLength` _output_get (`self.CameraDistance`))
        (set `SpringArmComponent.TargetArmLength` (`KismetMathLibrary.Lerp` 0.0 200.0 _returnvalue) (`self.CameraOffset`))))))

(fn `Convert Players to Locations`)

(fn `Get Players`
  (`KismetArrayLibrary.Array_Clear` (`self.Joined_PlayerActors`))
  (bind _outactors (`GameplayStatics.GetAllActorsOfClass` "/Game/Blueprints/Core/PC_Default.PC_Default_C"))
  (for _array_element _outactors
    (if (`/Game/Blueprints/Core/PC_Default.Joined` _array_element)
      (`KismetArrayLibrary.Array_Add` (`self.Joined_PlayerActors`) (`/Game/Blueprints/Core/PC_Default.Controller Pawn` _array_element))))
  (return))

(fn `UserConstructionScript`)