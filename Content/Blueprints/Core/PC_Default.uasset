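; Default player controller for drop-in/drop-out play on a shared level camera, with per-controller player info from the game instance.
; Join input toggles spawning or destroying a CH_Default, updating game mode lists and camera tracking, and copying health stats to PlayerInfo on leave.
; It references the character without possessing it, forwarding sticks each tick and dash, sword and lock-on presses as messages.
; The bottom face button messages overlapping interactables.
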(event `Key|Gamepad_FaceButton_Bottom`
  (params (Key :type "Key Structure"))
  (:`Pressed`
    (for _array_element (`self.GetOverlappingActors` (`self.Controller Pawn`) "/Game/Blueprints/Components/Component_Interactable.Component_Interactable_C")
      (message `/Game/Blueprints/Variables/Interfaces/Interface_Gameplay.Interact` _array_element))))

(event `Setup Controller`
  (`self.Setup Variables`))

(event `InputAction|Player Dash`
  (params (Key :type "Key Structure"))
  (:`Pressed`
    (message `/Game/Blueprints/Variables/Interfaces/Interface_Gameplay.Controller: Send Dash` (`self.Controller Pawn`))))

(event `self.ReceiveTick`
  (params (DeltaSeconds :type "Float (single-precision)"))
  (`/Engine/EditorBlueprintResources/StandardMacros.IsValid` (`self.Controller Pawn`)
    (:`Is Valid`
      (message `/Game/Blueprints/Variables/Interfaces/Interface_Gameplay.Controller: Send Left Joystick` (`self.Controller Pawn`) (`KismetMathLibrary.MakeVector2D` (`self.GetInputAxisValue`) (`self.GetInputAxisValue`)))
      (message `/Game/Blueprints/Variables/Interfaces/Interface_Gameplay.Controller: Send Right Joystick` (`self.Controller Pawn`) (`KismetMathLibrary.MakeVector2D` (`self.GetInputAxisValue`) (`self.GetInputAxisValue`))))))

(event `InputAction|Player Join`
  (params (Key :type "Key Structure"))
  (:`Pressed`
    (bind _joined (`/Game/Blueprints/Variables/Functions/FunctionLib.Controller Joined` self))
    (if _joined
      (`self.Player: Leave`)
      (else
        (`self.Player: Join`)))))

(event `InputAction|Player Sword`
  (params (Key :type "Key Structure"))
  (:`Pressed`
    (message `/Game/Blueprints/Variables/Interfaces/Interface_Gameplay.Controller: Send Left Face Button` (`self.Controller Pawn`) true))
  (:`Released`
    (message `/Game/Blueprints/Variables/Interfaces/Interface_Gameplay.Controller: Send Left Face Button` (`self.Controller Pawn`) false)))

(event `InputAction|Player Lock-On`
  (params (Key :type "Key Structure"))
  (:`Pressed`
    (message `/Game/Blueprints/Variables/Interfaces/Interface_Gameplay.Controller: Send Lock-On` (`self.Controller Pawn`) true))
  (:`Released`
    (message `/Game/Blueprints/Variables/Interfaces/Interface_Gameplay.Controller: Send Lock-On` (`self.Controller Pawn`) false)))

(fn `Camera: Possess`
  (`self.SetViewTargetWithBlend` self (`/Game/Blueprints/Core/GM_Default.Level Camera` (`self.Gamemode`)) 0.0 "VTBlend_Linear" 0.0 false))

(fn `Character: Set Control`
  (params (Character :type "/Game/Blueprints/Character/CH_Default Object Reference") (`Input Type` :type "/Game/Blueprints/Variables/Enum/Enum_InputSetups Enum" :default "NewEnumerator0"))
  (set `self.Controller Pawn` Character)
  (return))

(fn `Character: Spawn`
  (returns (Character :type "/Game/Blueprints/Character/CH_Default Object Reference"))
  (bind _returnvalue (`|SpawnActorFromClass` "/Game/Blueprints/Character/CH_Default.CH_Default_C" (`KismetMathLibrary.MakeTransform` (0.0 0.0 200.0)) "AlwaysSpawn" "OverrideRootScale" self null))
  (return _returnvalue))

(fn `Player: Join`
  (bind _character (`self.Character: Spawn`))
  (`self.Character: Set Control` _character)
  (message `/Game/Blueprints/Variables/Interfaces/Interface_Gameplay.Setup` (`self.Controller Pawn`) self)
  (set `self.Joined` true)
  (`KismetArrayLibrary.Array_Add` (`/Game/Blueprints/Core/GM_Default.Controllers Joined` (`self.Gamemode`)) self)
  (`KismetArrayLibrary.Array_Add` (`/Game/Blueprints/Core/GM_Default.Character Pawns` (`self.Gamemode`)) (cast `/Game/Blueprints/Character/CH_Default` (`self.Controller Pawn`) :!pure true))
  (`/Game/Blueprints/Camera/Camera_Default.Camera: Update Players` (`/Game/Blueprints/Core/GM_Default.Level Camera` (`self.Gamemode`)) true (`self.Controller Pawn`)))

(fn `Player: Leave`
  ;[0 0 0 0.5] Save Stats from dropping out
  (setmembers `/Game/Blueprints/Variables/Struct/Player/Struct_PlayerInfo` :`StructRef` (`self.Player Info`) :`Stats` (`/Game/Blueprints/Components/Component_Health.Stats` (`/Game/Blueprints/Character/CH_Default.Component_Health` (cast `/Game/Blueprints/Character/CH_Default` (`self.Controller Pawn`) :!pure true))))
  (`/Game/Blueprints/Camera/Camera_Default.Camera: Update Players` (`/Game/Blueprints/Core/GM_Default.Level Camera` (`self.Gamemode`)) false (`self.Controller Pawn`))
  (set `self.Joined` false)
  (`KismetArrayLibrary.Array_RemoveItem` (`/Game/Blueprints/Core/GM_Default.Controllers Joined` (`self.Gamemode`)) self)
  (`KismetArrayLibrary.Array_RemoveItem` (`/Game/Blueprints/Core/GM_Default.Character Pawns` (`self.Gamemode`)) (cast `/Game/Blueprints/Character/CH_Default` (`self.Controller Pawn`) :!pure true))
  (`self.K2_DestroyActor` (`self.Controller Pawn`)))

(fn `Setup Variables`
  (set `self.Gamemode` (cast `/Game/Blueprints/Core/GM_Default` (`GameplayStatics.GetGameMode`) :!pure true))
  (set `self.Instance` (cast `/Game/Blueprints/Core/Instance_Default` (`GameplayStatics.GetGameInstance`) :!pure true))
  (bind _output_get (set `self.Controller Index` (`GameplayStatics.GetPlayerControllerID` self)))
  (set `self.Player Info` (`|GetArrayItem` (`/Game/Blueprints/Core/Instance_Default.Players` (`self.Instance`)) _output_get)))

(fn `UserConstructionScript`)