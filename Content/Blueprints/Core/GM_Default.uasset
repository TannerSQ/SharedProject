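; GM_Default is the default game mode that initializes a local multiplayer level with a shared camera.
; On BeginPlay it removes existing players and pawns, creates and stores local PC_Default controllers for four players, then runs their variable setup.
; It spawns a Camera_Default as player 0's view target, then notifies every actor implementing Interface_General that level setup is complete.
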(event `self.ReceiveBeginPlay`
  (`self.Level Loaded`))

(event `Level Loaded`
  (`self.Remove Players`)
  (`self.Create Controllers`)
  (`self.Setup Controllers`)
  (`self.Create Camera`)
  (`self.Level Setup`))

(event `Level Setup`
  (bind _outactors (`GameplayStatics.GetAllActorsWithInterface` "/Game/Blueprints/Variables/Interfaces/Interface_General.Interface_General_C"))
  (for _array_element _outactors
    (message `/Game/Blueprints/Variables/Interfaces/Interface_General.Level Setup Complete` _array_element)))

(fn `Create Camera`
  (bind _returnvalue (`|SpawnActorFromClass` "/Game/Blueprints/Camera/Camera_Default.Camera_Default_C" (`KismetMathLibrary.MakeTransform` (0.0 0.0 0.0)) "Undefined" "OverrideRootScale" null null))
  (`PlayerController.SetViewTargetWithBlend` (`GameplayStatics.GetPlayerController` 0) _returnvalue 0.0 "VTBlend_Linear" 0.0 false)
  (set `self.Level Camera` _returnvalue)
  (return))

(fn `Create Controllers`
  (for _index (range 4)
    (bind _returnvalue (`GameplayStatics.CreatePlayer` _index))
    (bind _aspc_default (cast `/Game/Blueprints/Core/PC_Default` _returnvalue))
    (`KismetArrayLibrary.Array_Add` (`self.Controllers`) _aspc_default))
  (return))

(fn `Remove Players`
  (bind _outactors (`GameplayStatics.GetAllActorsOfClass` (`self.PlayerControllerClass`)))
  (for _array_element _outactors
    (`GameplayStatics.RemovePlayer` _array_element true))
  (return))

(fn `Setup Controllers`
  (for _array_element (`self.Controllers`)
    (`/Game/Blueprints/Core/PC_Default.Setup Variables` _array_element))
  (return))

(fn `UserConstructionScript`)