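; Interactable zone used as a child actor, giving its parent a proximity-based interaction with a face button prompt.
; A sphere tracks CH_Default overlaps, notifying the parent as occupancy starts or ends and popping the widget in or out, with a reminder animation for extra overlaps.
; Interact calls are forwarded to the parent only while interactable.
; Button icon, prompt height and radius are configurable.
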(event `self.ReceiveBeginPlay`
  (bind _output_get (set `self.Button UI` (cast `/Game/UI/Buttons/UI_FaceButton` (`WidgetComponent.GetUserWidgetObject` (`self.Widget`)) :!pure true)))
  (`Image.SetBrushFromTexture` (`/Game/UI/Buttons/UI_FaceButton.Button` _output_get) (select `/Game/Blueprints/Variables/Enum/Enum_FaceButtons` (`self.Button`) :`NewEnumerator0` "/Game/UI/Buttons/Textures/Button_Y.Button_Y" :`NewEnumerator1` "/Game/UI/Buttons/Textures/Button_X.Button_X" :`NewEnumerator2` "/Game/UI/Buttons/Textures/Button_B.Button_B" :`NewEnumerator3` "/Game/UI/Buttons/Textures/Button_A.Button_A" :!type "Texture2D Object Reference") false))

(event `self.Interaction Radius.OnComponentBeginOverlap`
  (params (OverlappedComponent :type "PrimitiveComponent Object Reference") (OtherActor :type "Actor Object Reference") (OtherComp :type "PrimitiveComponent Object Reference") (OtherBodyIndex :type Integer) (bFromSweep :type Boolean) (SweepResult :type "HitResult Structure (by ref)"))
  (bind _button_ui (`self.Button UI`))
  (if (== (`KismetArrayLibrary.Array_Length` (`PrimitiveComponent.GetOverlappingActors` (`self.Interaction Radius`) "/Game/Blueprints/Character/CH_Default.CH_Default_C")) 1)
    (bind _output_get (set `self.bInteractable` true))
    (`self.Interactable` _output_get)
    (else
      (`UserWidget.PlayAnimation` _button_ui (`/Game/UI/Buttons/UI_FaceButton.Remind` _button_ui) 0.0 1 "Forward" 1.0 false))))

(event `self.Interaction Radius.OnComponentEndOverlap`
  (params (OverlappedComponent :type "PrimitiveComponent Object Reference") (OtherActor :type "Actor Object Reference") (OtherComp :type "PrimitiveComponent Object Reference") (OtherBodyIndex :type Integer))
  (if (== (`KismetArrayLibrary.Array_Length` (`PrimitiveComponent.GetOverlappingActors` (`self.Interaction Radius`) "/Game/Blueprints/Character/CH_Default.CH_Default_C")) 0)
    (bind _output_get (set `self.bInteractable` false))
    (`self.Interactable` _output_get)))

(event `Interactable`
  (params (True :type Boolean))
  (bind _button_ui (`self.Button UI`))
  (message `/Game/Blueprints/Variables/Interfaces/Interface_Gameplay.Inside Zone` (`self.GetParentActor`) True)
  (`UserWidget.PlayAnimation` _button_ui (`/Game/UI/Buttons/UI_FaceButton.Pop` _button_ui) 0.0 1 (select `bool` True :`false` "Reverse" :`true` "Forward" :!type "EUMGSequencePlayMode Enum") 1.0 false))

(event `/Game/Blueprints/Variables/Interfaces/Interface_Gameplay.Interact`
  (if (`self.bInteractable`)
    (message `/Game/Blueprints/Variables/Interfaces/Interface_Gameplay.Interact` (`self.GetParentActor`))))

(fn `UserConstructionScript`
  (set `SpringArmComponent.TargetArmLength` (`self.Button Height`) (`self.Height`))
  (`SphereComponent.SetSphereRadius` (`self.Interaction Radius`) (`self.Radius`) false))