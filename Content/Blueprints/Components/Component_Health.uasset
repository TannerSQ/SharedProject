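; Health component that applies incoming combat damage to its owner's health stat.
; The damage event divides the amount by the current defense level, then subtracts the result from current health.
; At zero or below it sends a health-depleted message to the owner.
; Otherwise it spawns a floating damage widget at the owner's projected screen position, offset vertically, so killing blows show no number.
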(event `/Game/Blueprints/Variables/Interfaces/Interface_Gameplay.Combat: Damage`
  (params (Damage :type "/Game/Blueprints/Variables/Struct/Damage/Struct_Damage Structure") (Actor :type "Actor Object Reference"))
  (bind _screenposition (`WidgetLayoutLibrary.ProjectWorldLocationToWidgetPosition` (`GameplayStatics.GetPlayerController` 0) (`Actor.K2_GetActorLocation` (`self.GetOwner`)) true))
  (bind _new_damage (`self.Damage Filter: Armor` Damage_Damage_2_7F42294249DD718E60575FA0A3BF6F70))
  (set `self.Damage` _new_damage)
  (bind _structout (setmembers `/Game/Blueprints/Variables/Struct/Player/Struct_PlayerStats_Health` :`StructRef` (`.Health_18_F51CC52549E2E2DDAC1D57BA2DE104C8` (break `/Game/Blueprints/Variables/Struct/Damage/Struct_AttackableStats` (`self.Stats`))) :`Current Health` (- (`.CurrentHealth_4_30139DE541793FC158D49DA87600ACC7` (break `/Game/Blueprints/Variables/Struct/Player/Struct_PlayerStats_Health` (`.Health_18_F51CC52549E2E2DDAC1D57BA2DE104C8` (break `/Game/Blueprints/Variables/Struct/Damage/Struct_AttackableStats` (`self.Stats`))))) _new_damage)))
  (if (<= (break `/Game/Blueprints/Variables/Struct/Player/Struct_PlayerStats_Health` _structout) 0.0)
    (message `/Game/Blueprints/Variables/Interfaces/Interface_Gameplay.Combat: Health Depleted` (`self.GetOwner`))
    (else
      (bind _returnvalue (`|CreateWidget` "/Game/UI/Combat/UI_HitDMG.UI_HitDMG_C" (`GameplayStatics.GetPlayerController` 0)))
      (`CanvasPanelSlot.SetPosition` (`WidgetLayoutLibrary.SlotAsCanvasSlot` (`/Game/UI/Combat/UI_HitDMG.DMGText` _returnvalue)) (`KismetMathLibrary.MakeVector2D` (`KismetMathLibrary.BreakVector2D` _screenposition) (+ (`.Y` (`KismetMathLibrary.BreakVector2D` _screenposition)) (* (`self.Hit UI Offset`) -1.0))))
      (`UserWidget.AddToViewport` _returnvalue 0)
      (`/Game/UI/Combat/UI_HitDMG.Play` _returnvalue (`self.Damage`)))))

(fn `Damage Filter: Armor`
  (params (Damage :type "Float (double-precision)"))
  (returns (`New Damage` :type "Float (double-precision)"))
  (bind _defense_currentdefenselevel (break `/Game/Blueprints/Variables/Struct/Player/Struct_PlayerInfo_Defense` (break `/Game/Blueprints/Variables/Struct/Damage/Struct_AttackableStats` (`self.Stats`))))
  (return (/ Damage (`KismetMathLibrary.Conv_IntToDouble` _defense_currentdefenselevel))))