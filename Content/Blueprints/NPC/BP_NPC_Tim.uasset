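; BP_NPC_Tim is an NPC whose interaction plays a short scripted dialogue and camera tour, with his line announcing a pan over to a cave area.
; TriggerInteraction pauses the players, shows the line, then steps NPC camera focus through five positions in sequence with fixed delays between them.
; Focus stays off the players until the final step returns it and unpauses them, using NPC helper functions not defined here.
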(event `self.Trigger Interaction`
  (`self.NPC: Pause Players` true)
  (`self.NPC: Dialogue` "Hey! I'm gonna do some talking.... Then I'm gonna pan over to that cave area")
  (`KismetSystemLibrary.Delay` 1.0)
  (`self.NPC: Camera Focus` 0)
  (`KismetSystemLibrary.Delay` 1.0)
  (`self.NPC: Camera Focus` 1)
  (`KismetSystemLibrary.Delay` 1.0)
  (`self.NPC: Camera Focus` 2)
  (`KismetSystemLibrary.Delay` 1.0)
  (`self.NPC: Camera Focus` 3)
  (`KismetSystemLibrary.Delay` 1.0)
  (`self.NPC: Camera Focus` 4)
  (`KismetSystemLibrary.Delay` 1.0)
  (`self.NPC: Return Focus to Players`)
  (`self.NPC: Pause Players` false))

(fn `UserConstructionScript`
  (`parent.UserConstructionScript`))