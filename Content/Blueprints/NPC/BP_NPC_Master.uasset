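; Base NPC Blueprint that handles player interaction, camera focus, damage and pausing player movement.
; Caches the game mode's LevelCamera after level setup, points it at the NPC on Interact, and releases it on leaving the zone or on request.
; An overlap with CH_Default fires the empty TriggerInteraction event, damage goes to ComponentHealth, and pausing broadcasts through Interface_Gameplay.
; Dialogue only prints text, CameraFocus and Animation are empty, and older camera-blend logic is disconnected.
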(event `self.Interaction Overlap.OnComponentBeginOverlap`
  (params (OverlappedComponent :type "PrimitiveComponent Object Reference") (OtherActor :type "Actor Object Reference") (OtherComp :type "PrimitiveComponent Object Reference") (OtherBodyIndex :type Integer) (bFromSweep :type Boolean) (SweepResult :type "HitResult Structure (by ref)"))
  (cast `/Game/Blueprints/Character/CH_Default` OtherActor)
  (`self.Trigger Interaction`))

(event `Trigger Interaction`)

(event `/Game/Blueprints/Variables/Interfaces/Interface_General.Level Setup Complete`
  (set `self.Player Camera` (`/Game/Blueprints/Core/GM_Default.Level Camera` (cast `/Game/Blueprints/Core/GM_Default` (`GameplayStatics.GetGameMode`) :!pure true))))

(event `NPC: Dialogue`
  (params (Text :type String))
  (`KismetSystemLibrary.PrintString` Text))

(event `NPC: Camera Focus`
  (params (`Camera Position` :type Integer) (`Return focus to Players` :type Boolean)))

(event `NPC: Animation`)

(event `NPC: Return Focus to Players`
  (set `/Game/Blueprints/Camera/Camera_Default.Focus Camera on Location` false (`self.Player Camera`)))

(event `/Game/Blueprints/Variables/Interfaces/Interface_Gameplay.Combat: Damage`
  (params (Damage :type "/Game/Blueprints/Variables/Struct/Damage/Struct_Damage Structure") (Actor :type "Actor Object Reference"))
  (`/Game/Blueprints/Components/Component_Health.Combat: Damage` (`self.Component_Health`) Damage null))

(event `NPC: Pause Players`
  (params (Pause :type Boolean))
  (bind _outactors (`GameplayStatics.GetAllActorsWithInterface` "/Game/Blueprints/Variables/Interfaces/Interface_Gameplay.Interface_Gameplay_C"))
  (for _array_element _outactors
    (message `/Game/Blueprints/Variables/Interfaces/Interface_Gameplay.Players: Stop Moving` _array_element Pause)))

(event `/Game/Blueprints/Variables/Interfaces/Interface_Gameplay.Interact`
  (bind (_returnvalue_x _returnvalue_y) (`KismetMathLibrary.BreakVector` (`SceneComponent.K2_GetComponentLocation` (`self.DefaultSceneRoot`))))
  (set `/Game/Blueprints/Camera/Camera_Default.Location_CameraFocus` (`KismetMathLibrary.MakeVector` _returnvalue_x _returnvalue_y) (`self.Player Camera`))
  (set `/Game/Blueprints/Camera/Camera_Default.Focus Camera on Location` true (`self.Player Camera`)))

(event `/Game/Blueprints/Variables/Interfaces/Interface_Gameplay.Inside Zone`
  (params (Entered :type Boolean))
  (if (not Entered)
    (set `/Game/Blueprints/Camera/Camera_Default.Focus Camera on Location` false (`self.Player Camera`))))

(fn `UserConstructionScript`)